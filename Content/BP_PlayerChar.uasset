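; BP_PlayerChar is a player-controlled actor that moves in discrete steps and quarter turns, driven by raw key events.
; W and S offset it forward or backward by MoveDist along its current rotation, with sweep collision.
; A adds positive 90-degree yaw (a right turn) and D the opposite, both applied instantly.
; BeginPlay, Tick, overlap and construction logic are empty.
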(event EventBeginPlay)

(event Collision|EventActorBeginOverlap
  (params (OtherActor :type Actor%20Object%20Reference)))

(event EventTick
  (params (DeltaSeconds :type Float%20%28single-precision%29)))

(event Input|KeyboardEvents|E
  (params (Key :type Key%20Structure :default "None")))

(event Input|KeyboardEvents|A
  (params (Key :type Key%20Structure :default "None"))
  (:Pressed
    (Transformation|AddActorLocalRotation (Math|Rotator|MakeRotator 0.0 0.0 9e+01) false false)))

(event Input|KeyboardEvents|D
  (params (Key :type Key%20Structure :default "None"))
  (:Pressed
    (Transformation|AddActorLocalRotation (Math|Rotator|MakeRotator 0.0 0.0 -9e+01) false false)))

(event Input|KeyboardEvents|W
  (params (Key :type Key%20Structure :default "None"))
  (:Pressed
    (Transformation|AddActorWorldOffset (Math|Vector|RotateVector (* (Variables|Default|GetMoveDist) (Class|KismetMathLibrary|VectorForward)) (Transformation|GetActorRotation)) true)))

(event Input|KeyboardEvents|S
  (params (Key :type Key%20Structure :default "None"))
  (:Pressed
    (Transformation|AddActorWorldOffset (Math|Vector|RotateVector (* (Variables|Default|GetMoveDist) (Class|KismetMathLibrary|VectorBackward)) (Transformation|GetActorRotation)) true)))

(fn ConstructionScript)