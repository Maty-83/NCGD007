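; BP_Crusher is a crusher hazard that resets the level through GM_GameModeBase when it registers a hit.
; The construction script caches the game mode for that call.
; Tick calls MoveUpDown, which is unfinished: its DirUp branch does nothing, and the offset, speed and MinZ/MaxZ nodes are unconnected, so the crusher does not move.
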(event EventBeginPlay)

(event Collision|EventActorBeginOverlap
  (params (OtherActor :type Actor%20Object%20Reference)))

(event EventTick
  (params (DeltaSeconds :type Float%20%28single-precision%29))
  (CallFunction|MoveUpDown DeltaSeconds))

(event Collision|EventHit
  (params (MyComp :type Primitive%20Component%20Object%20Reference) (Other :type Actor%20Object%20Reference) (OtherComp :type Primitive%20Component%20Object%20Reference) (bSelfMoved :type Boolean) (HitLocation :type Vector :default "0, 0, 0") (HitNormal :type Vector :default "0, 0, 0") (NormalImpulse :type Vector :default "0, 0, 0") (Hit :type Hit%20Result%20Structure%20%28by%20ref%29))
  (Default|ResetLevel (Variables|Default|GetGameMode)))

(fn ConstructionScript
  (bind _asgm_game_mode_base (Utilities|Casting|CastToGM_GameModeBase (Game|GetGameMode)))
  (Variables|Default|SetGameMode _asgm_game_mode_base))

(fn MoveUpDown
  (params (DeltaSeconds :type Float%20%28double-precision%29))
  (if (Variables|Default|GetDirUp)
    _))